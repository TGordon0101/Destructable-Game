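; BP_HousesRemain is a display Blueprint that shows a houses remaining figure as 3D text in the game.
; On BeginPlay it caches a cast reference to the VRGameMode.
; Every Tick it sets the Text3D text from the game mode's Score scaled down by a fixed divisor, minus its HousesRemaining variable.
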(event EventBeginPlay
  (bind _asvrgame_mode (Utilities|Casting|CastToVRGameMode (Game|GetGameMode)))
  (Variables|Default|SetAs%20VRGame%20Mode _asvrgame_mode))

(event EventTick
  (params (DeltaSeconds :type Float%20%28single-precision%29))
  (Class|Text3DComponent|SetText (Variables|Default|GetText3D) (Utilities|Text|ToText(Float) (- (/ (Variables|/Game/VRTemplate/Blueprints/VRGameMode.VRGameMode_C|GetScore (Variables|Default|GetAs%20VRGame%20Mode)) 2e+02) (Variables|Default|GetHouses%20Remaining)) "HalfToEven")))

(fn ConstructionScript)