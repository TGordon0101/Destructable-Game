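; BP_ROOFING is a roof building piece that detects when its TestRoof component has fallen.
; BeginPlay stores the roof's starting world location.
; Each Tick compares the current height to that start, and once it drops more than 100 units below, clears IsStanding and prints a debug "Hello" message.
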(event EventBeginPlay
  (Variables|Default|SetInitial%20Location (Transformation|GetWorldLocation (Variables|Default|GetTestRoof))))

(event EventTick
  (params (DeltaSeconds :type Float%20%28single-precision%29))
  (if (< (.z (Transformation|GetWorldLocation (Variables|Default|GetTestRoof))) (- (.z (Variables|Default|GetInitial%20Location)) 1e+02))
    (Variables|Default|SetIsStanding false)
    (Development|PrintString "Hello")))

(fn ConstructionScript)