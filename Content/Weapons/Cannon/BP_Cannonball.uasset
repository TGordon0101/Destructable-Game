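; Cannonball projectile that destroys geometry collection buildings in the VR cannon game and scores the hit.
; On hit against a geometry collection component while its Break flag is set, it spawns a short-lived FS_MasterField field at the impact to fracture the target, then clears the flag.
; Each break raises the VRGameMode score, decrements the remaining house count with a debug print, and plays a debris sound.
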(event Custom|Break%20Geometry
  (params (SpawnTransform :type Transform))
  (bind _returnvalue (Game|SpawnActorfromClass "/Engine/EditorResources/FieldNodes/FS_MasterField.FS_MasterField_C" SpawnTransform "Undefined" 0 0))
  (Actor|SetLifeSpan _returnvalue 0.1)
  (bind _asvrgame_mode (Utilities|Casting|CastToVRGameMode (Variables|Default|GetGameMode)))
  (Default|ScoreGoesUp _asvrgame_mode)
  (bind _result (Math|Integer|DecrementInt (Variables|/Game/VRTemplate/Blueprints/VRGameMode.VRGameMode_C|GetHouses%20Remaining _asvrgame_mode))
    (:%20%20
      (Development|PrintString (Utilities|String|ToString(Integer) _result))
      (Audio|PlaySoundatLocation "/Game/Asstes/SFX_Music/Debris/Bluezone_BC0277_debris_falling_rock_urban_002__Bluezone_Corp_.Bluezone_BC0277_debris_falling_rock_urban_002__Bluezone_Corp_" (Transformation|GetWorldLocation (Variables|Default|GetCannonBall self)) "0, 0, 0" 1.0 1.0 0.0 0 0 0 0))))

(event EventBeginPlay
  (Variables|Default|SetGameMode (Game|GetGameMode)))

(event Collision|EventHit
  (params (MyComp :type Primitive%20Component%20Object%20Reference) (Other :type Actor%20Object%20Reference) (OtherComp :type Primitive%20Component%20Object%20Reference) (bSelfMoved :type Boolean) (HitLocation :type Vector :default "0, 0, 0") (HitNormal :type Vector :default "0, 0, 0") (NormalImpulse :type Vector :default "0, 0, 0") (Hit :type Hit%20Result%20Structure%20%28by%20ref%29))
  (if (Variables|Default|GetBreak)
    (if (== OtherComp "/Script/GeometryCollectionEngine.GeometryCollectionComponent")
      (CallFunction|BreakGeometry (Math|Conversions|ToTransform(Vector) (Transformation|GetWorldLocation MyComp)))
      (Variables|Default|SetBreak false))))

(fn ConstructionScript)