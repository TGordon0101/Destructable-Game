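; Cannon actor that is aimed and fired through grab components, launching BP_Cannonball projectiles.
; Grabbing a direction control sets a half-second move flag; Tick then yaws body and base or rolls Aim1.
; Grabbing the wick spawns a ball at Aim, impulses it along FirePoint-to-Aim, and spawns BP_Ammo at its saved location.
; Firing clears CanFire, which this graph never resets, although the wick reappears after FireRate.
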(event OnGrabbed(GrabComponent)
  (if (Variables|Default|GetCanFire)
    (CallFunction|FireCannon)
    (Variables|Default|SetCanFire false)
    (Rendering|SetVisibility (Variables|Default|GetWick) false false)
    (Utilities|FlowControl|Delay (Variables|Default|GetFireRate))
    (Rendering|SetVisibility (Variables|Default|GetWick) true false)))

(event OnGrabbed(GrabRight)
  (bind _right (Variables|Default|GetRight))
  (Variables|Default|SetMoveRight true)
  (Rendering|SetVisibility _right false false)
  (Utilities|FlowControl|Delay 0.5)
  (Variables|Default|SetMoveRight false)
  (Rendering|SetVisibility _right true false))

(event OnGrabbed(GrabLeft)
  (bind _left (Variables|Default|GetLeft))
  (Variables|Default|SetMoveLeft true)
  (Rendering|SetVisibility _left false false)
  (Utilities|FlowControl|Delay 0.5)
  (Variables|Default|SetMoveLeft false)
  (Rendering|SetVisibility _left true false))

(event OnGrabbed(GrabDown)
  (bind _down (Variables|Default|GetDown))
  (Variables|Default|SetMoveDown true)
  (Rendering|SetVisibility _down false false)
  (Utilities|FlowControl|Delay 0.5)
  (Variables|Default|SetMoveDown false)
  (Rendering|SetVisibility _down true false))

(event OnGrabbed(GrabUp)
  (bind _up (Variables|Default|GetUp))
  (Variables|Default|SetMoveUp true)
  (Rendering|SetVisibility _up false false)
  (Utilities|FlowControl|Delay 0.5)
  (Variables|Default|SetMoveUp false)
  (Rendering|SetVisibility _up true false))

(event Custom|Fire%20Cannon
  (bind _aim (Variables|Default|GetAim))
  (bind _returnvalue (Transformation|GetWorldLocation _aim))
  (bind _returnvalue_2 (Game|SpawnActorfromClass "/Game/Weapons/Cannon/BP_Cannonball.BP_Cannonball_C" (Math|Conversions|ToTransform(Vector) _returnvalue) "Undefined" 0 0))
  (Physics|AddImpulse (Variables|/Game/Weapons/Cannon/BP_Cannonball.BP_Cannonball_C|GetCannonBall _returnvalue_2) (* (Math|Vector|Normalize (- _returnvalue (Transformation|GetWorldLocation (Variables|Default|GetFirePoint)))) (Variables|Default|GetCannonForce)) "None" false)
  (Game|SpawnActorfromClass "/Game/Weapons/Cannon/BP_Ammo.BP_Ammo_C" (Math|Conversions|ToTransform(Vector) (Variables|Default|GetAmmo%20Location)) "Undefined" 0 0))

(event EventBeginPlay
  (Variables|Default|SetAmmo%20Location (Transformation|GetWorldLocation (Variables|Default|GetBP_Ammo))))

(event EventTick
  (params (DeltaSeconds :type Float%20%28single-precision%29))
  (CallFunction|RotateLR)
  (CallFunction|RotateUD))

(fn ConstructionScript)

(fn RotateLR
  (bind _cannon_base_weapon (Variables|Default|Getcannon_base_weapon))
  (bind _cannon_body_weapon (Variables|Default|Getcannon_body_weapon))
  (bind _returnvalue (Transformation|GetRelativeTransform _cannon_base_weapon))
  (bind _returnvalue_2 (Transformation|GetRelativeTransform _cannon_body_weapon))
  (if (Variables|Default|GetMoveRight)
    (Variables|Default|SetRotDir 0.1)
    (Transformation|SetRelativeLocationAndRotation _cannon_body_weapon (.location _returnvalue_2) (Math|Rotator|MakeRotator (.roll (.rotation _returnvalue_2)) (.pitch (.rotation _returnvalue_2)) (+ (.yaw (.rotation _returnvalue_2)) (Variables|Default|GetRotDir))) false false :!label _label)
    (Transformation|SetRelativeLocationAndRotation _cannon_base_weapon (.location _returnvalue) (Math|Rotator|MakeRotator (.roll (.rotation _returnvalue)) (.pitch (.rotation _returnvalue)) (+ (.yaw (.rotation _returnvalue)) (Variables|Default|GetRotDir))) false false)
    (Variables|Default|SetRotDir 0.0)
    (elif (Variables|Default|GetMoveLeft)
      (Variables|Default|SetRotDir -0.1)
      (goto _label))))

(fn RotateUD
  (bind _aim1 (Variables|Default|GetAim1))
  (bind _returnvalue (Transformation|GetRelativeTransform _aim1))
  (if (Variables|Default|GetMoveDown)
    (Variables|Default|SetRotDir 0.1)
    (Transformation|SetRelativeLocationAndRotation _aim1 (.location _returnvalue) (Math|Rotator|MakeRotator (+ (.roll (.rotation _returnvalue)) (Variables|Default|GetRotDir)) (.pitch (.rotation _returnvalue)) (.yaw (.rotation _returnvalue))) false false :!label _label)
    (Variables|Default|SetRotDir 0.0)
    (elif (Variables|Default|GetMoveUp)
      (Variables|Default|SetRotDir -0.1)
      (goto _label))))