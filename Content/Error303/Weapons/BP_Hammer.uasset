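; BP_Hammer is a throwable hammer weapon that breaks geometry collections on impact.
; Throw_Hammer applies an impulse to the static mesh along the Bottom-to-Top axis, with a debug line trace whose hit distance is only printed.
; When a Hit matches the geometry collection component, BreakGeometry spawns a short-lived FS_MasterField at the impact point to trigger destruction.
; An unconnected trace-distance check never runs.
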(event Custom|Throw_Hammer
  (bind _bottom (Variables|Default|GetBottom))
  (bind _staticmesh (Variables|Default|GetStaticMesh))
  (bind _top (Variables|Default|GetTop))
  (bind _returnvalue (Transformation|GetWorldLocation _bottom))
  (bind _returnvalue_2 (Transformation|GetWorldLocation _staticmesh))
  (bind _returnvalue_3 (Transformation|GetWorldLocation _top))
  (bind _returnvalue_4 (Math|Vector|GetUnitDirection(Vector) _returnvalue_3 _returnvalue))
  (bind _returnvalue_5 (* _returnvalue_4 "5000.000000,5000.000000,5000.000000"))
  (bind _returnvalue_6 (* _returnvalue_5 "-1.000000,-1.000000,-1.000000"))
  (bind _outhit (Collision|LineTraceByChannel _returnvalue_2 (+ _returnvalue_2 _returnvalue_6) "TraceTypeQuery1" false 0 "ForDuration"))
  (Development|PrintString (Utilities|String|ToString(Float) (.Distance (Collision|BreakHitResult _outhit))))
  (Physics|AddImpulse (Variables|Default|GetStaticMesh) _returnvalue_6 "None" false))

(event Custom|Break%20Geometry
  (params (SpawnTransform :type Transform))
  (bind _returnvalue (Game|SpawnActorfromClass "/Engine/EditorResources/FieldNodes/FS_MasterField.FS_MasterField_C" SpawnTransform "Undefined" 0 0))
  (Actor|SetLifeSpan _returnvalue 0.1))

(event Collision|EventHit
  (params (MyComp :type Primitive%20Component%20Object%20Reference) (Other :type Actor%20Object%20Reference) (OtherComp :type Primitive%20Component%20Object%20Reference) (bSelfMoved :type Boolean) (HitLocation :type Vector :default "0, 0, 0") (HitNormal :type Vector :default "0, 0, 0") (NormalImpulse :type Vector :default "0, 0, 0") (Hit :type Hit%20Result%20Structure%20%28by%20ref%29))
  (if (== OtherComp "/Script/GeometryCollectionEngine.GeometryCollectionComponent")
    (CallFunction|BreakGeometry (Math|Conversions|ToTransform(Vector) HitLocation))
    (Development|PrintString "Hello")))

(fn ConstructionScript)